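; BP_TestSpawner is a test actor that places a pooled BP_BasicBullet at its own location about once per second.
; On BeginPlay it caches the game instance cast to MainGameInstance.
; Tick accumulates delta time, then fetches a bullet from the game instance's object pool, moves it to the spawner and resets the timer, rather than spawning new actors.
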(event `self.ReceiveBeginPlay`
  (bind _asmain_game_instance (cast `MainGameInstance` (`GameplayStatics.GetGameInstance`)))
  (set `self.Main Game Instance` _asmain_game_instance))

(event `self.ReceiveTick`
  (params (DeltaSeconds :type "Float (single-precision)"))
  (bind _output_get (set `self.Timer` (+ DeltaSeconds (`self.Timer`))))
  (if (> _output_get 1.0)
    (bind _returnvalue (`MainGameInstance.FetchFromPool` (`self.Main Game Instance`) "/Game/DanTestBPs/BP_BasicBullet.BP_BasicBullet_C"))
    (`self.K2_SetActorLocation` _returnvalue (`self.K2_GetActorLocation`) false false)
    (set `self.Timer` 0.0)))

(fn `UserConstructionScript`)