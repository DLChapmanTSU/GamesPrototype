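; BP_BasicBullet is a simple projectile that damages the player on contact.
; Tick moves it along its forward vector at Speed using a swept SetActorLocation, without a movement component.
; Sphere overlaps ignore components tagged CollisionIgnore; any other overlap destroys the bullet.
; If the overlapped actor is a PlayerPawnAlpha with a StatsManager, it first deals 1 damage through that component.
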(event `self.ReceiveTick`
  (params (DeltaSeconds :type "Float (single-precision)"))
  (`self.K2_SetActorLocation` (+ (`self.K2_GetActorLocation`) (* (`self.GetActorForwardVector`) (* (`self.Speed`) DeltaSeconds))) true))

(event `self.Sphere.OnComponentBeginOverlap`
  (params (OverlappedComponent :type "PrimitiveComponent Object Reference") (OtherActor :type "Actor Object Reference") (OtherComp :type "PrimitiveComponent Object Reference") (OtherBodyIndex :type Integer) (bFromSweep :type Boolean) (SweepResult :type "HitResult Structure (by ref)"))
  (if (not (`KismetArrayLibrary.Array_Contains` (`ActorComponent.ComponentTags` OtherComp) "CollisionIgnore"))
    (bind _asplayer_pawn_alpha (cast `/Game/Multiplayer/PlayerPawnAlpha` OtherActor)
      (:`then`
        (bind _returnvalue (`self.GetComponentByClass` _asplayer_pawn_alpha "/Script/GamesPrototype.StatsManager"))
        (`/Engine/EditorBlueprintResources/StandardMacros.IsValid` _returnvalue
          (:`Is Valid`
            (`StatsManager.DealDamage` _returnvalue 1))
          (:`Is Not Valid`
            _)))
      (:`CastFailed`
        _))
    (`self.K2_DestroyActor`)))

(fn `UserConstructionScript`)