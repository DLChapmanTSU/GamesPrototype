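; BP_ResourceBox is a spinning, tilted pickup box that grants PlayerPawnAlpha a resource, healing or buff on overlap.
; Overlaps require an AttackManager and ignore components tagged CollisionIgnore.
; ResourceType selects the effect: AttackManager adds resources or sets the retain buff, while StatsManager heals health and radiation or sets the armour buff.
; Once used, it debug-prints the type, invalidates it and hides the cube rather than destroying the actor.
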(event `self.ReceiveTick`
  (params (DeltaSeconds :type "Float (single-precision)"))
  (`self.K2_SetActorRotation` (`KismetMathLibrary.MakeRotator` 20.0 (.pitch (`self.K2_GetActorRotation`)) (.yaw (`self.K2_GetActorRotation`))))
  (`self.K2_AddActorWorldRotation` (`KismetMathLibrary.MakeRotator` 0.0 0.0 (* DeltaSeconds 99.0))))

(event `self.Box.OnComponentBeginOverlap`
  (params (OverlappedComponent :type "PrimitiveComponent Object Reference") (OtherActor :type "Actor Object Reference") (OtherComp :type "PrimitiveComponent Object Reference") (OtherBodyIndex :type Integer) (bFromSweep :type Boolean) (SweepResult :type "HitResult Structure (by ref)"))
  (bind _returnvalue (`self.GetComponentByClass` OtherActor "/Script/GamesPrototype.StatsManager"))
  (bind _returnvalue_2 (`self.GetComponentByClass` OtherActor "/Script/GamesPrototype.AttackManager"))
  (bind _resource_type (`self.Resource Type`))
  (if (== (`GameplayStatics.GetObjectClass` OtherActor) "/Game/Multiplayer/PlayerPawnAlpha.PlayerPawnAlpha_C")
    (if (not (`KismetArrayLibrary.Array_Contains` (`ActorComponent.ComponentTags` OtherComp) "CollisionIgnore"))
      (`/Engine/EditorBlueprintResources/StandardMacros.IsValid` _returnvalue_2
        (:`Is Valid`
          (switch `int` (`self.Resource Type`)
            (:`0`
              (`AttackManager.AddResource` _returnvalue_2 _resource_type :!label _label))
            (:`1`
              (goto _label))
            (:`2`
              (`/Engine/EditorBlueprintResources/StandardMacros.IsValid` _returnvalue
                (:`Is Valid`
                  (`StatsManager.HealHealth` _returnvalue 5)
                  (`StatsManager.HealRadiation` _returnvalue 10))
                (:`Is Not Valid`
                  _)))
            (:`3`
              (`/Engine/EditorBlueprintResources/StandardMacros.IsValid` _returnvalue
                (:`Is Valid`
                  (`StatsManager.SetArmourBuff` _returnvalue))
                (:`Is Not Valid`
                  _)))
            (:`4`
              (`/Engine/EditorBlueprintResources/StandardMacros.IsValid` _returnvalue_2
                (:`Is Valid`
                  (`AttackManager.SetRetainBuff` _returnvalue_2))
                (:`Is Not Valid`
                  _))))
          (`KismetSystemLibrary.PrintString` (`KismetStringLibrary.Conv_IntToString` _resource_type))
          (set `self.Resource Type` -1)
          (`SceneComponent.SetVisibility` (`self.Cube`) false true))))))

(fn `UserConstructionScript`)