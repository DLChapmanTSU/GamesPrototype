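; BP_TazerBullet is a tazer projectile actor that flies straight along its forward vector at Speed, moved each Tick with a swept SetActorLocation.
; When its sphere overlaps a component not tagged CollisionIgnore, it spawns a Tazereffecthandler at its transform and destroys itself.
; An unreachable branch would deal damage through the player's StatsManager, and a CustomEvent function duplicates the Tick movement.
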(event `self.ReceiveTick`
  (params (DeltaSeconds :type "Float (single-precision)"))
  (`self.K2_SetActorLocation` (+ (`self.K2_GetActorLocation`) (* (`self.GetActorForwardVector`) (* (`self.Speed`) DeltaSeconds))) true))

(event `self.Sphere.OnComponentBeginOverlap`
  (params (OverlappedComponent :type "PrimitiveComponent Object Reference") (OtherActor :type "Actor Object Reference") (OtherComp :type "PrimitiveComponent Object Reference") (OtherBodyIndex :type Integer) (bFromSweep :type Boolean) (SweepResult :type "HitResult Structure (by ref)"))
  (if (not (`KismetArrayLibrary.Array_Contains` (`ActorComponent.ComponentTags` OtherComp) "CollisionIgnore"))
    (`|SpawnActorFromClass` "/Game/Multiplayer/tazer/tazereffecthandler.tazereffecthandler_C" (`self.GetTransform`) "Undefined" "MultiplyWithRoot" null null)
    (`self.K2_DestroyActor`)))

(fn `CustomEvent`
  (params (DeltaSeconds :type "Float (single-precision)"))
  (`self.K2_SetActorLocation` (+ (`self.K2_GetActorLocation`) (* (`self.GetActorForwardVector`) (* (`self.Speed`) DeltaSeconds))) true))

(fn `UserConstructionScript`)